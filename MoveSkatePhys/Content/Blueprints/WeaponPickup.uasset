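; Weapon pickup that shows a randomly chosen gun mesh, spinning and bobbing on a sine wave above its base.
; On first PlayerRoller overlap, it sets the side weapon with full default ammo, then switches from the revolver or replaces the held gun's child actor class.
; It then destroys the mesh and plays a sound.
; Reset rerolls the gun and re-arms pickup, but only while the mesh is valid.
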(event `self.ReceiveBeginPlay`
  (set `self.GunID` (`KismetMathLibrary.RandomInteger` 2))
  (bind _returnvalue (`AddComponent|NODE_AddSkeletalMeshComponent-1` :`RelativeTransform` (`KismetMathLibrary.Conv_VectorToTransform` (`KismetMathLibrary.MakeVector` 0.0 0.0 (`self.ZOffsetFromBase`)))))
  (bind _output_get (set `self.Mesh` _returnvalue))
  (`SkinnedMeshComponent.SetSkinnedAssetAndUpdate` _output_get (`|GetArrayItem` (`self.Meshes`) (`self.GunID`)) true))

(event `self.ReceiveTick`
  (params (DeltaSeconds :type "Float (single-precision)"))
  (if (`KismetSystemLibrary.IsValid` (stale `self.ReceiveBeginPlay` _output_get))
    (`SceneComponent.K2_AddWorldRotation` (stale `self.ReceiveBeginPlay` _output_get) (`KismetMathLibrary.MakeRotator` 0.0 0.0 (* DeltaSeconds (`self.RotationSpeed`))) false false)
    (`SceneComponent.K2_SetWorldLocation` (stale `self.ReceiveBeginPlay` _output_get) (+ (`KismetMathLibrary.MakeVector` 0.0 0.0 (* (`KismetMathLibrary.DegSin` (* (`KismetSystemLibrary.GetGameTimeInSeconds`) (`self.Float Frequency`))) (`self.Float Amplitude`))) (`self.FloatAnchor`)) false false)
    (set `self.FloatAnchor` (+ (`KismetMathLibrary.MakeVector` 0.0 0.0 (`self.ZOffsetFromBase`)) (`SceneComponent.K2_GetComponentLocation` (`self.StaticMesh`))))))

(event `self.ReceiveActorBeginOverlap`
  (params (OtherActor :type "Actor Object Reference"))
  (bind _output (`|GetArrayItem` (`self.GunTypes`) (`self.GunID`)))
  (bind (_isfiring _current_ammo _maxammo _clipsize) (defaults `/Game/FirstPersonBP/Guns/DiscLauncher_Gun` _output))
  (bind _asplayer_roller (cast `/Game/Blueprints/PlayerRoller` OtherActor))
  (`/Engine/EditorBlueprintResources/StandardMacros.DoOnce` false :!label _label
    (:`Completed`
      (set `/Game/Blueprints/PlayerRoller.Side Weapon` (make `/Game/FirstPersonBP/Guns/GunVariables` _output _clipsize _maxammo) _asplayer_roller)
      (bind _gun (`/Game/Blueprints/PlayerRoller.Gun` _asplayer_roller))
      (if (== (`ChildActorComponent.ChildActorClass` _gun) "/Game/FirstPersonBP/Guns/Revolver_Gun.Revolver_Gun_C")
        (`/Game/Blueprints/PlayerRoller.SwitchWeapons` _asplayer_roller)
        (else
          (`ChildActorComponent.SetChildActorClass` _gun _output)))
      (`ActorComponent.K2_DestroyComponent` (stale `self.ReceiveBeginPlay` _output_get))
      (`GameplayStatics.PlaySound2D` "/Game/Sounds/Disk_launcher_pick_up.Disk_launcher_pick_up" 1.0 1.0 0.0 null null))))

(event `Reset`
  (bind _mesh (`self.Mesh`))
  (if (`KismetSystemLibrary.IsValid` _mesh)
    (`ActorComponent.K2_DestroyComponent` _mesh)
    (set `self.GunID` (`KismetMathLibrary.RandomInteger` 2))
    (bind _returnvalue (`AddComponent|NODE_AddSkeletalMeshComponent-2`))
    (bind _output_get (set `self.Mesh` _returnvalue))
    (`SkinnedMeshComponent.SetSkinnedAssetAndUpdate` _output_get (`|GetArrayItem` (`self.Meshes`) (`self.GunID`)) true)
    (goto _label :!via `Reset`)))

(fn `UserConstructionScript`)