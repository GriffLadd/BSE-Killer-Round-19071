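; BouncePad is a jump pad that launches a PlayerRoller when it overlaps the actor.
; On overlap it keeps the roller's horizontal velocity and resets the vertical component, so incoming fall speed does not affect the bounce.
; It then applies a fixed, mass-dependent impulse along the Box's up vector, so rotating the Box aims the launch.
; A Boosting sound plays at the Box's location with attenuation.
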(event `self.ReceiveActorBeginOverlap`
  (params (OtherActor :type "Actor Object Reference"))
  (bind _box (`self.Box`))
  (bind _asplayer_roller (cast `/Game/Blueprints/PlayerRoller` OtherActor))
  (bind _roller (`/Game/Blueprints/PlayerRoller.Roller` _asplayer_roller))
  (bind _returnvalue (`PrimitiveComponent.GetPhysicsLinearVelocity` _roller "None"))
  (`PrimitiveComponent.SetPhysicsLinearVelocity` _roller (`KismetMathLibrary.MakeVector` (.x _returnvalue) (.y _returnvalue)) false "None")
  (`PrimitiveComponent.AddImpulse` (`/Game/Blueprints/PlayerRoller.Roller` _asplayer_roller) (* (`KismetMathLibrary.GetUpVector` (`SceneComponent.K2_GetComponentRotation` _box)) 50000.0) "None" false)
  (`GameplayStatics.PlaySoundAtLocation` "/Game/Sounds/Boosting.Boosting" (`SceneComponent.K2_GetComponentLocation` _box) (struct) 1.0 1.0 0.0 "/Game/Attentuation.Attentuation" null null))

(fn `UserConstructionScript`)