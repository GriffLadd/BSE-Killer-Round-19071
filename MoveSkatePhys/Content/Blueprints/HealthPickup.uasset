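; Health pickup actor that restores an overlapping PlayerRoller to max health, hides its orb and plays a 2D pickup sound.
; A DoOnce limits it to a single use until the Reset event shows the orb again and re-arms it.
; Tick bobs the orb on a sine wave of game time around an anchor offset vertically from the static mesh's location.
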(event `Reset`
  (`SceneComponent.SetVisibility` (`self.Orb`) true false)
  (goto _label :!via `Reset`))

(event `self.ReceiveActorBeginOverlap`
  (params (OtherActor :type "Actor Object Reference"))
  (bind _asplayer_roller (cast `/Game/Blueprints/PlayerRoller` OtherActor))
  (`/Engine/EditorBlueprintResources/StandardMacros.DoOnce` false :!label _label
    (:`Completed`
      (set `/Game/Blueprints/PlayerRoller.Health` (`/Game/Blueprints/PlayerRoller.MaxHealth` _asplayer_roller) _asplayer_roller)
      (`SceneComponent.SetVisibility` (`self.Orb`) false false)
      (`GameplayStatics.PlaySound2D` "/Game/Sounds/Disk_launcher_pick_up.Disk_launcher_pick_up" 1.0 1.0 0.0 null null))))

(event `self.ReceiveTick`
  (params (DeltaSeconds :type "Float (single-precision)"))
  (bind _orb (`self.Orb`))
  (if (`KismetSystemLibrary.IsValid` _orb)
    (`SceneComponent.K2_SetWorldLocation` _orb (+ (`KismetMathLibrary.MakeVector` 0.0 0.0 (* (`KismetMathLibrary.DegSin` (* (`KismetSystemLibrary.GetGameTimeInSeconds`) (`self.Float Frequency`))) (`self.Float Amplitude`))) (`self.FloatAnchor`)) false false)
    (set `self.FloatAnchor` (+ (`KismetMathLibrary.MakeVector` 0.0 0.0 (`self.ZOffsetFromBase`)) (`SceneComponent.K2_GetComponentLocation` (`self.StaticMesh`))))))

(fn `UserConstructionScript`)