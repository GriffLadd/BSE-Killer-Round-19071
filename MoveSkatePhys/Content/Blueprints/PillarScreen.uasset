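; PillarScreen is an in-game display actor that shows the current score and an elapsed time readout.
; Every Tick it casts the game mode to KillerRoundGameMode and copies its Score into the Score text.
; The Time text shows the actor's own time since creation, formatted as a time string, rather than a timer from the game mode.
; Neither text updates if the cast fails.
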(event `self.ReceiveTick`
  (params (DeltaSeconds :type "Float (single-precision)"))
  (bind _askiller_round_game_mode (cast `/Game/KillerRoundGameMode` (`GameplayStatics.GetGameMode`)))
  (`TextRenderComponent.K2_SetText` (`self.Score`) (`KismetTextLibrary.Conv_DoubleToText` (`/Game/KillerRoundGameMode.Score` _askiller_round_game_mode) "HalfToEven"))
  (`TextRenderComponent.K2_SetText` (`self.Time`) (`KismetTextLibrary.Conv_StringToText` (`KismetStringLibrary.TimeSecondsToString` (`self.GetGameTimeSinceCreation`)))))

(fn `UserConstructionScript`)